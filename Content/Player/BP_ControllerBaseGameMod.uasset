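; Player controller for the base game mode that drives a BP_Camera actor with a visible mouse cursor.
; On BeginPlay it adds the base Enhanced Input context and caches the camera and all BP_BaseUnit actors.
; Input actions pan, yaw and vertically zoom the camera.
; Walk only stores the cursor hit location in CurrentCommand, as the unit move loop and effect spawn are disconnected.
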(event Input|EnhancedActionEvents|EnhancedInputActionIA_Walk
  (params (ActionValue :type Boolean) (ElapsedSeconds :type Float%20%28double-precision%29) (TriggeredSeconds :type Float%20%28double-precision%29) (InputAction :type Input%20Action%20Object%20Reference :default "/Game/Player/IA_Walk.IA_Walk"))
  ;[1 1 1] Move all tims to location
  (Variables|Default|SetCurrentCommand (.Location (Collision|BreakHitResult (.HitResult (Game|Player|GetHitResultUnderCursorbyChannel "TraceTypeQuery1" true))))))

(event Input|EnhancedActionEvents|EnhancedInputActionIA_Move
  (params (ActionValue :type Vector%202D%20Structure) (ElapsedSeconds :type Float%20%28double-precision%29) (TriggeredSeconds :type Float%20%28double-precision%29) (InputAction :type Input%20Action%20Object%20Reference :default "/Game/Player/IA_Move.IA_Move"))
  (bind (_x _y) (Math|Vector2D|BreakVector2D ActionValue))
  (bind _camerabasegamemod (Variables|Default|GetCameraBaseGameMod))
  ;[1 1 1] Camera movement
  (Pawn|Input|AddMovementInput _camerabasegamemod (Transformation|GetActorForwardVector) _y false)
  (Pawn|Input|AddMovementInput _camerabasegamemod (Transformation|GetActorRightVector) _x false))

(event Input|EnhancedActionEvents|EnhancedInputActionIA_Rotate
  (params (ActionValue :type Vector%202D%20Structure) (ElapsedSeconds :type Float%20%28double-precision%29) (TriggeredSeconds :type Float%20%28double-precision%29) (InputAction :type Input%20Action%20Object%20Reference :default "/Game/Player/IA_Rotate.IA_Rotate"))
  (bind (_x _y) (Math|Vector2D|BreakVector2D ActionValue))
  (bind _camerabasegamemod (Variables|Default|GetCameraBaseGameMod))
  ;[1 1 1] Camera movement
  (Class|Actor|AddActorWorldRotation _camerabasegamemod (Math|Rotator|MakeRotator 0.0 0.0 _x))
  (Class|Actor|AddActorWorldRotation _camerabasegamemod (Math|Rotator|MakeRotator 0.0 0.0 _y)))

(event Input|EnhancedActionEvents|EnhancedInputActionIA_Zoom
  (params (ActionValue :type Float%20%28double-precision%29) (ElapsedSeconds :type Float%20%28double-precision%29) (TriggeredSeconds :type Float%20%28double-precision%29) (InputAction :type Input%20Action%20Object%20Reference :default "/Game/Player/IA_Zoom.IA_Zoom"))
  ;[1 1 1] Camera movement
  (Transformation|AddActorWorldOffset (Variables|Default|GetCameraBaseGameMod) (Math|Vector|MakeVector 0.0 0.0 (* ActionValue 45.0))))

(event EventTick
  (params (DeltaSeconds :type Float%20%28single-precision%29)))

(event EventBeginPlay
  (Variables|Default|SetbShowMouseCursor true)
  (Input|AddMappingContext (PlayerController|LocalPlayerSubsystems|GetEnhancedInputLocalPlayerSubsystem (Game|GetPlayerController 0)) "/Game/Player/IMC_BaseInput.IMC_BaseInput" 0 "(bIgnoreAllPressedKeysUntilRelease=True,bForceImmediately=False,bNotifyUserSettings=False)")
  (bind _returnvalue (Actor|GetActorOfClass "/Game/Player/BP_Camera.BP_Camera_C"))
  (Variables|Default|SetCameraBaseGameMod _returnvalue)
  (bind _outactors (Actor|GetAllActorsOfClass "/Game/Characters/GreenTim/BP_BaseUnit.BP_BaseUnit_C"))
  (Variables|Default|SetUnits _outactors))

(fn ConstructionScript)